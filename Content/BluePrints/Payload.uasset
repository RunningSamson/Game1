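; Payload actor that travels along the spline of a referenced track actor, such as an escort-style payload.
; On BeginPlay, if ActivePayload is set, MovePayload plays a timeline at a rate of one over Duration, starting from PayloadStartOffset.
; Each update lerps the timeline alpha over the spline length and sets the actor's world location and rotation at that distance.
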(event `self.ReceiveBeginPlay`
  (if (`self.ActivePayload`)
    (`self.MovePayload`)))

(event `MovePayload`
  (bind _returnvalue (`KismetMathLibrary.Lerp` 0.0 (`SplineComponent.GetSplineLength` (`/Game/BluePrints/Track.PayloadSpline` (`self.TrackRef`))) (`self.Alpha`)))
  (`TimelineComponent.SetPlayRate` (`self.PayloadMover`) (/ 1.0 (`self.Duration`)))
  (`TimelineComponent.SetNewTime` (`self.PayloadMover`) (`self.PayloadStartOffset`))
  (bind (_direction _alpha) (`Timeline|PayloadMover`)
    (:`Update`
      (set `self.Alpha` _alpha)
      (`self.K2_SetActorLocationAndRotation` (`SplineComponent.GetLocationAtDistanceAlongSpline` (`/Game/BluePrints/Track.PayloadSpline` (`self.TrackRef`)) _returnvalue "World") (`SplineComponent.GetRotationAtDistanceAlongSpline` (`/Game/BluePrints/Track.PayloadSpline` (`self.TrackRef`)) _returnvalue "World")))))

(fn `UserConstructionScript`)