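; Payload actor that travels along a referenced track's spline while something overlaps its sphere, like an escort-objective cart.
; Sphere overlap plays the PayloadMover timeline, whose rate is set from Duration; ending overlap stops it in place.
; Each timeline update maps Alpha to distance along the spline and sets the actor's world location and rotation.
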(event `self.Sphere.OnComponentBeginOverlap`
  (params (OverlappedComponent :type "PrimitiveComponent Object Reference") (OtherActor :type "Actor Object Reference") (OtherComp :type "PrimitiveComponent Object Reference") (OtherBodyIndex :type Integer) (bFromSweep :type Boolean) (SweepResult :type "HitResult Structure (by ref)"))
  (set `self.ActivePayload` true)
  (if (`self.ActivePayload`)
    (`self.MovePayload`)))

(event `MovePayload`
  (bind (_direction _alpha) (`Timeline|PayloadMover` :!label _label)
    (:`Update`
      (set `self.Alpha` _alpha)
      (`self.BeginLocation`))))

(event `self.ReceiveBeginPlay`
  (`TimelineComponent.SetPlayRate` (`self.PayloadMover`) (/ 1.0 (`self.Duration`)))
  (`TimelineComponent.SetNewTime` (`self.PayloadMover`) (`self.PayloadStartOffset`))
  (goto _label :!via `SetNewTime`))

(event `StopPayload`
  (goto _label :!via `Stop`))

(event `self.Sphere.OnComponentEndOverlap`
  (params (OverlappedComponent :type "PrimitiveComponent Object Reference") (OtherActor :type "Actor Object Reference") (OtherComp :type "PrimitiveComponent Object Reference") (OtherBodyIndex :type Integer))
  (set `self.ActivePayload` false)
  (set `self.Alpha` 0.0)
  (goto _label :!via `Stop`))

(fn `BeginLocation`
  (bind _returnvalue (`KismetMathLibrary.Lerp` 0.0 (`SplineComponent.GetSplineLength` (`/Game/BluePrints/Track.PayloadSpline` (`self.TrackRef`))) (`self.Alpha`)))
  (`self.K2_SetActorLocationAndRotation` (`SplineComponent.GetLocationAtDistanceAlongSpline` (`/Game/BluePrints/Track.PayloadSpline` (`self.TrackRef`)) _returnvalue "World") (`SplineComponent.GetRotationAtDistanceAlongSpline` (`/Game/BluePrints/Track.PayloadSpline` (`self.TrackRef`)) _returnvalue "World")))

(fn `UserConstructionScript`)