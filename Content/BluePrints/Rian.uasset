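; Rian is a player-controlled pawn Blueprint that handles basic movement and mouse look.
; Forward/back and left/right axis inputs add movement along the Camera component's world forward and right vectors, so movement follows the view direction.
; MouseX and MouseY feed controller yaw and pitch directly, and the construction script is empty.
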(event `InputAxis|Forward_backward`
  (params (AxisValue :type "Float (single-precision)"))
  ;[1 1 1] Movement
  (`self.AddMovementInput` (`KismetMathLibrary.GetForwardVector` (`SceneComponent.K2_GetComponentRotation` (`self.Camera`))) AxisValue))

(event `InputAxis|Left_Right`
  (params (AxisValue :type "Float (single-precision)"))
  ;[1 1 1] Movement
  (`self.AddMovementInput` (`KismetMathLibrary.GetRightVector` (`SceneComponent.K2_GetComponentRotation` (`self.Camera`))) AxisValue))

(event `InputAxis|MouseY`
  (params (AxisValue :type "Float (single-precision)"))
  ;[1 1 1] Axis looking
  (`self.AddControllerPitchInput` AxisValue))

(event `InputAxis|MouseX`
  (params (AxisValue :type "Float (single-precision)"))
  ;[1 1 1] Axis looking
  (`self.AddControllerYawInput` AxisValue))

(fn `UserConstructionScript`)